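; BP_VRChar is a VR player pawn that keeps itself upright on a Cesium globe, apparently a VR moon.
; BeginPlay and Possessed snap local up to the ellipsoid normal; BeginPlay also adds the input mapping context.
; Possessed also finds the GeoRefsManager and prints moon-relative and actor up vectors for debugging.
; IA_Move drives camera-relative movement, while an authority/remote setup branch is left unconnected.
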(event `self.ReceiveBeginPlay`
  (`CesiumGlobeAnchorComponent.SnapLocalUpToEllipsoidNormal` (`self.CesiumGlobeAnchor`))
  (bind _aspawn_controller (cast `PawnController` (`GameplayStatics.GetPlayerController` 0))
    (:`then`
      (`EnhancedInputSubsystemInterface.AddMappingContext` (pcsubsystem `EnhancedInputLocalPlayerSubsystem` _aspawn_controller) "/Game/Pawns/Inputs/Game/IMC_VRChar.IMC_VRChar" 0 (struct)))
    (:`CastFailed`
      (`KismetSystemLibrary.PrintString` "BP_VRChar: Failed to cast player controller as PawnController."))))

(event `self.ReceivePossessed`
  (params (NewController :type "Controller Object Reference"))
  (bind _returnvalue (`GameplayStatics.GetActorOfClass` "/Script/ArtemisOutpost.GeoRefsManager"))
  (bind _output_get (set `self.GRM` _returnvalue))
  (`self.SetGeoRefsManager` _output_get)
  (if (`KismetSystemLibrary.IsValid` (`self.GeoRefsManager`))
    (`CesiumGlobeAnchorComponent.SnapLocalUpToEllipsoidNormal` (`self.CesiumGlobeAnchor`))
    (bind _returnvalue_2 (`GeoRefsManager.GetVRMoon` (`self.GeoRefsManager`)))
    (`KismetSystemLibrary.PrintString` (`KismetStringLibrary.Concat_StrStr` "VRChar: Raw calculated UP Vector: " (`KismetStringLibrary.Conv_VectorToString` (`KismetMathLibrary.Normal` (- (`self.K2_GetActorLocation`) (`self.K2_GetActorLocation` _returnvalue_2))))))
    (`KismetSystemLibrary.PrintString` (`KismetStringLibrary.Concat_StrStr` "VRChar: Actor up Vector: " (`KismetStringLibrary.Conv_VectorToString` (`KismetMathLibrary.Normal` (`KismetMathLibrary.GetUpVector` (`self.K2_GetActorRotation`))))))
    (else
      (`KismetSystemLibrary.PrintString` "VP_VRChar: GeoRefsManager not initilized."))))

(event `EnhancedInput|/Game/Pawns/Inputs/Game/Actions/VR/IA_Move`
  (params (ActionValue :type "Vector2D Structure") (ElapsedSeconds :type "Float (double-precision)") (TriggeredSeconds :type "Float (double-precision)") (InputAction :type "InputAction Object Reference" :default "/Game/Pawns/Inputs/Game/Actions/VR/IA_Move.IA_Move"))
  (bind _vrcamera (`self.VRCamera`))
  (:`Triggered`
    (`self.AddMovementInput` (`KismetMathLibrary.Vector_Normal2D` (`SceneComponent.GetRightVector` _vrcamera)) ActionValue_X)
    (`self.AddMovementInput` (`KismetMathLibrary.Vector_Normal2D` (`SceneComponent.GetForwardVector` _vrcamera)) ActionValue_Y)))

(fn `UserConstructionScript`)