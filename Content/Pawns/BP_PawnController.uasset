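; Player controller that switches between an AR pawn and a VR character on a Cesium-based Moon with rovers.
; On IA_SwitchMode the client changes tracking origin, input mapping, world-to-meters scale and visibility, then RunOnServer possesses the target pawn.
; Entering VR first teleports the character beside the master rover via georeference conversion and aligns it to the surface.
; It also registers the rover with the camera manager and submits area scans.
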(event `self.ReceiveBeginPlay`
  (set `self.CurrentXRMode` "AR"))

(event `RunOnClient`
  (bind _returnvalue (`GameplayStatics.GetActorOfClass` "/Script/ArtemisOutpost.CustomCesiumCameraManager"))
  (`CustomCesiumCameraManager.AddNewMasterRover` _returnvalue (`self.MasterRover`)))

(event `EnhancedInput|/Game/Pawns/Inputs/Game/Actions/IA_SwitchMode`
  (params (ActionValue :type Boolean) (ElapsedSeconds :type "Float (double-precision)") (TriggeredSeconds :type "Float (double-precision)") (InputAction :type "InputAction Object Reference" :default "/Game/Pawns/Inputs/Game/Actions/IA_SwitchMode.IA_SwitchMode"))
  (bind _arpawn (`self.ARPawn`))
  (bind _arpawn_2 (`self.ARPawn`))
  (bind _masterrover (`self.MasterRover`))
  (bind _masterrover_2 (`self.MasterRover`))
  (bind _vrpawn (`self.VRPawn`))
  (bind _vrpawn_2 (`self.VRPawn`))
  (bind _vrpawn_3 (`self.VRPawn`))
  (:`Started`
    ; Client-side mode switch. Triggers OnRep_CurrentXRMode
    (switch `EXRMode` (`self.CurrentXRMode`)
      (:`VR`
        (bind _output_get (set `self.CurrentXRMode` "AR"))
        (`KismetSystemLibrary.LogString` (`KismetStringLibrary.Concat_StrStr` "[CLIENT]: Switched to mode: " (`|GetEnumeratorNameAsString` _output_get)))
        (`CharVR.SetIsPossessed` (`self.VRPawn`) false)
        (`HeadMountedDisplayFunctionLibrary.SetTrackingOrigin` "Stage")
        (`EnhancedInputSubsystemInterface.AddMappingContext` (pcsubsystem `EnhancedInputLocalPlayerSubsystem` self) "/Game/Pawns/Inputs/Game/IMC_ARRover.IMC_ARRover" 0 (struct))
        (`CharVR.SetShouldReplicateTransform` (`self.VRPawn`) false)
        ; Resize the XR World scale
        (`HeadMountedDisplayFunctionLibrary.SetWorldToMetersScale` (`self.CachedWTMValue`))
        ; Show / hide VRPawn + VRMoon
        (bind _returnvalue (`CharVR.GetVRTileset` _vrpawn))
        (`self.SetActorHiddenInGame` _returnvalue true)
        (`self.SetActorHiddenInGame` _vrpawn true)
        (`self.SetActorHiddenInGame` _masterrover true)
        (bind _returnvalue_2 (`MasterRover.GetPuppetRover` _masterrover))
        (`self.SetActorHiddenInGame` _returnvalue_2 false)
        (bind _returnvalue_3 (`PawnAR.GetARTileset` _arpawn))
        (`self.SetActorHiddenInGame` _returnvalue_3 false)
        (`self.SetActorHiddenInGame` _arpawn false)
        (`self.RunOnServer` :!label _label) ; TODO: we have to wait top ticks before calling this
      )
      (:`AR`
        (bind _output_get_2 (set `self.CurrentXRMode` "VR"))
        (`KismetSystemLibrary.LogString` (`KismetStringLibrary.Concat_StrStr` "[CLIENT]: Switched to mode: " (`|GetEnumeratorNameAsString` _output_get_2)))
        (`CharVR.SetIsPossessed` (`self.VRPawn`) true)
        (`HeadMountedDisplayFunctionLibrary.SetTrackingOrigin` "LocalFloor")
        (`EnhancedInputSubsystemInterface.AddMappingContext` (pcsubsystem `EnhancedInputLocalPlayerSubsystem` self) "/Game/Pawns/Inputs/Game/IMC_VRChar.IMC_VRChar" 0 (struct))
        (`CharVR.SetShouldReplicateTransform` (`self.VRPawn`) true)
        (set `self.CachedWTMValue` (`HeadMountedDisplayFunctionLibrary.GetWorldToMetersScale`))
        (`HeadMountedDisplayFunctionLibrary.SetWorldToMetersScale` 100.0)
        (bind _returnvalue_4 (`CharVR.GetVRTileset` _vrpawn_2))
        (`self.SetActorHiddenInGame` _returnvalue_4 false)
        (`self.SetActorHiddenInGame` _vrpawn_2 false)
        (`self.SetActorHiddenInGame` _masterrover_2 false)
        (bind _returnvalue_5 (`MasterRover.GetPuppetRover` _masterrover_2))
        (`self.SetActorHiddenInGame` _returnvalue_5 true)
        (bind _returnvalue_6 (`PawnAR.GetARTileset` _arpawn_2))
        (`self.SetActorHiddenInGame` _returnvalue_6 true)
        (`self.SetActorHiddenInGame` _arpawn_2 true)
        (bind _teleportposition (`self.CalculateVRTeleportPos`)
          (:`Out`
            (`self.K2_SetActorLocation` _vrpawn_3 _teleportposition false false)
            (bind _asbp_vrchar (cast `/Game/Pawns/BP_VRChar` _vrpawn_3)
              (:`then`
                (`/Game/Pawns/BP_VRChar.AlignNormalWithSurface` _asbp_vrchar)
                (`KismetSystemLibrary.PrintString` (`KismetStringLibrary.Concat_StrStr` "BP_MasterRover [CLIENT]: Position of the Master Rover before repossession:  " (`KismetStringLibrary.Conv_VectorToString` (`self.K2_GetActorLocation` (`self.MasterRover`)))))
                (goto _label))
              (:`CastFailed`
                (`KismetSystemLibrary.PrintString` "BP_PawnController: Failed to cast to VP_VRChar on possession (switch to VR mode).")))))))))

(event `RunOnServer`
  (switch `EXRMode` (`self.CurrentXRMode`)
    (:`VR`
      (set `self.CurrentXRMode` "AR")
      (`KismetSystemLibrary.LogString` (`KismetStringLibrary.Concat_StrStr` "[SERVER]: Switched to mode: " (`|GetEnumeratorNameAsString` (`self.CurrentXRMode`))))
      (`self.Possess` (`self.ARPawn`)))
    (:`AR`
      (set `self.CurrentXRMode` "VR")
      (`KismetSystemLibrary.LogString` (`KismetStringLibrary.Concat_StrStr` "[SERVER]: Switched to mode: " (`|GetEnumeratorNameAsString` (`self.CurrentXRMode`))))
      (bind _asbp_vrchar (cast `/Game/Pawns/BP_VRChar` (`self.VRPawn`))
        (:`then`
          (`self.Possess` _asbp_vrchar) ; TODO: We have to wait here until the orientation of propages correctly to the client.
        )
        (:`CastFailed`
          (`KismetSystemLibrary.PrintString` "BP_PawnController: Failed to cast to VP_VRChar on possession (switch to VR mode)."))))))

(event `EnhancedInput|/Game/Pawns/Inputs/Game/Actions/VR/IA_ScanArea`
  (params (ActionValue :type Boolean) (ElapsedSeconds :type "Float (double-precision)") (TriggeredSeconds :type "Float (double-precision)") (InputAction :type "InputAction Object Reference" :default "/Game/Pawns/Inputs/Game/Actions/VR/IA_ScanArea.IA_ScanArea"))
  (:`Started`
    (bind _returnvalue (`GeoRefsManager.UECoordsToVRMoonCoords` (`self.GeoRefsManager`) (`self.K2_GetActorLocation` (`self.MasterRover`))))
    (`self.ServerAddAreaScan` (make `AreaScan` _returnvalue (make `ArtemisPlayer`)))))

(event `self.ReceiveTick`
  (params (DeltaSeconds :type "Float (single-precision)")))

(fn `OnRep_CurrentXRMode`
  (if (`self.bFirstModePropagation`)
    (set `self.bFirstModePropagation` false)
    (elif (`self.IsLocalController`)
      (`KismetSystemLibrary.LogString` (`KismetStringLibrary.Concat_StrStr` "[CLIENT]: Switched to mode: " (`|GetEnumeratorNameAsString` (`self.CurrentXRMode`))))
      (switch `EXRMode` (`self.CurrentXRMode`)
        (:`VR`
          (bind _returnvalue (`CharVR.GetVRTileset` (`self.VRPawn`)))
          (`self.SetActorHiddenInGame` _returnvalue false)
          (bind _returnvalue_2 (`PawnAR.GetARTileset` (`self.ARPawn`)))
          (`self.SetActorHiddenInGame` _returnvalue_2 true))
        (:`AR`
          (bind _returnvalue_3 (`CharVR.GetVRTileset` (`self.VRPawn`)))
          (`self.SetActorHiddenInGame` _returnvalue_3 true)
          (bind _returnvalue_4 (`PawnAR.GetARTileset` (`self.ARPawn`)))
          (`self.SetActorHiddenInGame` _returnvalue_4 false)))
      (else
        (`KismetSystemLibrary.LogString` (`KismetStringLibrary.Concat_StrStr` "[SERVER]: Switched to mode: " (`|GetEnumeratorNameAsString` (`self.CurrentXRMode`))))
        (switch `EXRMode` (`self.CurrentXRMode`)
          (:`VR`
            (bind _returnvalue_5 (`GeoRefsManager.VRMoonCoordsToUECoords` (`self.GeoRefsManager`) (`KismetMathLibrary.MakeVector` -20.12831 9.72126 5.0)))
            (`self.K2_SetActorLocation` (`self.VRPawn`) _returnvalue_5 false false)
            (`KismetSystemLibrary.PrintString` (`KismetStringLibrary.Concat_StrStr` "VR Char position before posses in WORLD coords: " (`KismetStringLibrary.Conv_VectorToString` (`self.K2_GetActorLocation` (`self.VRPawn`)))))
            (`self.Possess` (`self.VRPawn`)))
          (:`AR`
            (`self.Possess` (`self.ARPawn`))))))))

(fn `RegisterProxyCameraOnMasterRover`
  (`KismetSystemLibrary.PrintString` "BP_PawnController: Adding rover as proxy camera to Custom Cesium Camera Manager...")
  (bind _returnvalue (`GameplayStatics.GetActorOfClass` "/Script/ArtemisOutpost.CustomCesiumCameraManager"))
  (`CustomCesiumCameraManager.AddNewMasterRover` _returnvalue (`self.MasterRover`))
  (`self.RunOnClient`))

(fn `UserConstructionScript`)