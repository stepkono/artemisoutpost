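; BP_FogOfWarTester is a test Blueprint that registers an area scan at its owner's location, presumably to exercise fog of war.
; On BeginPlay it converts that location to VR Moon coordinates through the GeoRefsManager found in the level.
; It passes the position, with a default player authorship, to the MoonDataManager on ArtemisGameState.
; A failed game state cast only prints a placeholder debug string.
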(event `self.ReceiveBeginPlay`
  (bind _returnvalue (`GameplayStatics.GetActorOfClass` "/Script/ArtemisOutpost.GeoRefsManager"))
  (bind _returnvalue_2 (`GeoRefsManager.UECoordsToVRMoonCoords` _returnvalue (`Actor.K2_GetActorLocation` (`self.GetOwner`))))
  (bind _asartemis_game_state (cast `ArtemisGameState` (`GameplayStatics.GetGameState`))
    (:`then`
      (`MoonDataManager.AddNewAreaScan` (`ArtemisGameState.GetMoonDataManager` _asartemis_game_state) (make `AreaScan` _returnvalue_2 (make `ArtemisPlayer`))))
    (:`CastFailed`
      (`KismetSystemLibrary.PrintString` "asdfasdfasdfasdfasdfasdfasdfasdfasdfasdasdfsafdfsadasdffadsfsdaasfdfas"))))

(event `self.ReceiveTick`
  (params (DeltaSeconds :type "Float (single-precision)")))