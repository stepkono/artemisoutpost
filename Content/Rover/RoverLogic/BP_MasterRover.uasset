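; BP_MasterRover is the master rover actor on a Cesium-georeferenced VR moon, mirrored on clients by a puppet rover.
; On authority, BeginPlay snaps it to the ellipsoid normal and prints up vectors for debugging.
; On remotes, SpawnPuppetRover converts its location through VR moon coordinates into AR moon world space via GeoRefsManager, then spawns and stores BP_PuppetRover there.
; Tick only runs a resetting timer that triggers nothing.
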(event `self.ReceiveBeginPlay`
  (`/Engine/EditorBlueprintResources/ActorMacros.Switch Has Authority`
    (:`Authority`
      (`CesiumGlobeAnchorComponent.SnapLocalUpToEllipsoidNormal` (`self.CesiumGlobeAnchor`))
      (bind _returnvalue (`GeoRefsManager.GetVRMoon` (`self.GeoRefsManager`)))
      (`KismetSystemLibrary.PrintString` (`KismetStringLibrary.Concat_StrStr` "Raw calculated UP Vector: " (`KismetStringLibrary.Conv_VectorToString` (`KismetMathLibrary.Normal` (- (`self.K2_GetActorLocation`) (`self.K2_GetActorLocation` _returnvalue))))))
      (`KismetSystemLibrary.PrintString` (`KismetStringLibrary.Concat_StrStr` "Actor up Vector: " (`KismetStringLibrary.Conv_VectorToString` (`KismetMathLibrary.Normal` (`KismetMathLibrary.GetUpVector` (`self.K2_GetActorRotation`))))))
      (`KismetSystemLibrary.PrintString` (`KismetStringLibrary.Concat_StrStr` "Cesium surface normal:  " (`KismetStringLibrary.Conv_VectorToString` (`KismetMathLibrary.Normal` (`KismetMathLibrary.Quat_GetAxisZ` (`CesiumGlobeAnchorComponent.GetEastSouthUpRotation` (`self.CesiumGlobeAnchor`))))))))
    (:`Remote`
      (`self.SpawnPuppetRover`))))

(event `self.ReceiveTick`
  (params (DeltaSeconds :type "Float (single-precision)"))
  (bind _output_get (set `self.Seconds` (+ DeltaSeconds (`self.Seconds`))))
  (if (> _output_get 3.0)
    (set `self.Seconds` 0.0)))

(fn `UserConstructionScript`)