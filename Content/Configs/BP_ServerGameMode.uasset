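; Server game mode that spawns and registers each joining player's VR character and master rover pawns.
; On join, it spawns a VR character at the origin and a rover above the TargetPoint tagged by player count, using GeoRefsManager moon-coordinate conversion for the height offset.
; After validity logging, which only blocks on an invalid VR character, it initializes the PawnController and registers the pawns.
; Reconnecting players are re-initialized and re-registered with their saved pawns.
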(event `self.ReceiveBeginPlay`
  (`|ExecutionSequence`
    (:`then_0`
      (add `self.PlayerJoinDelegate` (delegate `PlayerJoinDelegate_Event`)))
    (:`then_1`
      (add `self.PlayerReconnectedDelegate` (delegate `PlayerReconnectedDelegate_Event`)))))

(event `PlayerJoinDelegate_Event` :!signature `self.PlayerJoinDelegate`
  (params (PawnController :type "PawnController Object Reference"))
  (bind _asbp_pawn_controller (cast `/Game/Pawns/BP_PawnController` PawnController)
    (:`then`
      (bind (_masterrover _vrplayer) (`self.SpawnPlayerPawns` _asbp_pawn_controller))
      (bind (_vrcharout _masterroverout) (`self.CehcForValidPawns` _masterrover _vrplayer)
        (:`Out`
          (`PawnController.InitializePawns` _asbp_pawn_controller _vrcharout _masterroverout)
          (`/Game/Pawns/BP_PawnController.RegisterProxyCameraOnMasterRover` _asbp_pawn_controller) ; Not sure if master rover will be available on client
          (`self.RegisterPlayerPawns` _asbp_pawn_controller _masterroverout _vrcharout))))
    (:`CastFailed`
      (`KismetSystemLibrary.PrintString` "BP_ServerGameMode: Failed to cast PawnControler as BP_PawnController."))))

(event `PlayerReconnectedDelegate_Event` :!signature `self.PlayerReconnectedDelegate`
  (params (PawnController :type "PawnController Object Reference") (PlayerData :type "ArtemisPlayer Structure"))
  (bind (_pawncontroller _playernumber _masterrover _vrchar) (break `ArtemisPlayer` PlayerData))
  (`PawnController.InitializePawns` _pawncontroller _vrchar _masterrover)
  (`self.RegisterPlayerPawns` _pawncontroller _masterrover _vrchar))

(fn `SpawnPlayerPawns`
  (params (PawnController :type "/Game/Pawns/BP_PawnController Object Reference"))
  (returns (MasterRover :type "/Game/Rover/RoverLogic/BP_MasterRover Object Reference") (VRPlayer :type "/Game/Pawns/BP_VRChar Object Reference"))
  (bind _vrplayer (`self.SpawnVRCharacter`)
    (:`Out`
      (bind _master (`self.SpawnRoverMaster` PawnController)
        (:`Out`
          (return _master _vrplayer))))))

(fn `UserConstructionScript`)